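; GameManager is a manager Blueprint that handles main menu and options menu display, plus game-start events.
; Each show event lazily creates its widget for player controller 0, caches the reference and re-adds it to the viewport on later calls.
; Showing the main menu also enables the mouse cursor.
; Continue is an empty stub, and NewGame calls OpenLevel with the level name left as None.
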(event `ShowMainMenu`
  ;[1 1 1] Show Main Menu
  (`/Engine/EditorBlueprintResources/StandardMacros.IsValid` (`self.MainMenuRef`)
    (:`Is Valid`
      (`UserWidget.AddToViewport` (`self.MainMenuRef`) 0))
    (:`Is Not Valid`
      (bind _returnvalue (`|CreateWidget` "/Game/UI/MainMenu.MainMenu_C" (`GameplayStatics.GetPlayerController` 0)))
      (bind _output_get (set `self.MainMenuRef` _returnvalue))
      (`UserWidget.AddToViewport` _output_get 0)))
  (set `PlayerController.bShowMouseCursor` true (`GameplayStatics.GetPlayerController` 0)))

(event `ShowOptionsMenu`
  ;[1 1 1] ShowOptions Menu
  (`/Engine/EditorBlueprintResources/StandardMacros.IsValid` (`self.OptionsMenuRef`)
    (:`Is Valid`
      (`UserWidget.AddToViewport` (`self.OptionsMenuRef`) 0))
    (:`Is Not Valid`
      (bind _returnvalue (`|CreateWidget` "/Game/UI/Options.Options_C" (`GameplayStatics.GetPlayerController` 0)))
      (bind _output_get (set `self.OptionsMenuRef` _returnvalue))
      (`UserWidget.AddToViewport` _output_get 0))))

(event `Continue`)

(event `NewGame`
  (`GameplayStatics.OpenLevel` "None"))