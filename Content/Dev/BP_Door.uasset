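; BP_Door is an interactable door that swings open and closed on its hinge.
; The Interaction event toggles a closed flag and plays or reverses a timeline, which interpolates the Hinge component's relative yaw between zero and DoorAngle.
; OutlineON and OutlineOFF switch the mesh's custom depth rendering and stencil value to drive an outline highlight.
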(event `/Game/Dev/I_Interaction.Interaction`
  (params (Normal :type "Vector Structure"))
  (if (`self.isDoorClosed`)
    (set `self.isDoorClosed` false)
    (bind (_direction _open_close) (`Timeline|Open/Close Door` :!label _label)
      (:`Update`
        (`SceneComponent.K2_SetRelativeRotation` (`self.Hinge`) (`KismetMathLibrary.MakeRotator` 0.0 0.0 (`KismetMathLibrary.Lerp` 0.0 (`self.DoorAngle`) _open_close)) false false)))
    (else
      (set `self.isDoorClosed` true)
      (goto _label :!via `Reverse`))))

(event `/Game/Dev/I_Interaction.OutlineON`
  (`PrimitiveComponent.SetRenderCustomDepth` (`self.Mesh`) true)
  (`PrimitiveComponent.SetCustomDepthStencilValue` (`self.Mesh`) 2))

(event `/Game/Dev/I_Interaction.OutlineOFF`
  (`PrimitiveComponent.SetRenderCustomDepth` (`self.Mesh`) false)
  (`PrimitiveComponent.SetCustomDepthStencilValue` (`self.Mesh`) 0))

(fn `UserConstructionScript`)