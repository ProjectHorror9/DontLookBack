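; First aid kit pickup that heals the first-person player character when interacted with.
; Interaction adds HealingValue to CurrentHealth without clamping, then destroys the kit, only if CurrentHealth differs from MaxHealth.
; OutlineON and OutlineOFF toggle the static mesh's custom depth rendering and stencil value for highlighting.
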(event `/Game/Dev/I_Interaction.Interaction`
  (params (Normal :type "Vector Structure"))
  (bind _asfirst_person_character (cast `/Game/Characters/Player/FirstPersonCharacter` (`GameplayStatics.GetPlayerPawn` 0)))
  (bind _currenthealth (`/Game/Characters/Player/FirstPersonCharacter.CurrentHealth` _asfirst_person_character))
  (if (!= (`/Game/Characters/Player/FirstPersonCharacter.MaxHealth` _asfirst_person_character) _currenthealth)
    (set `/Game/Characters/Player/FirstPersonCharacter.CurrentHealth` (+ _currenthealth (`self.HealingValue`)) _asfirst_person_character)
    (`self.K2_DestroyActor`)))

(event `/Game/Dev/I_Interaction.OutlineON`
  (bind _staticmesh (`self.StaticMesh`))
  (`PrimitiveComponent.SetRenderCustomDepth` _staticmesh true)
  (`PrimitiveComponent.SetCustomDepthStencilValue` _staticmesh 2))

(event `/Game/Dev/I_Interaction.OutlineOFF`
  (bind _staticmesh (`self.StaticMesh`))
  (`PrimitiveComponent.SetRenderCustomDepth` _staticmesh false)
  (`PrimitiveComponent.SetCustomDepthStencilValue` _staticmesh 0))

(fn `UserConstructionScript`)